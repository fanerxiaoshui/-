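; Player slime character for a side-scroller that moves, jumps, splits off a body and recombines with it.
; Holding left mouse slows time and previews an aim from the cursor projected onto the character's plane; release calls Split, scaled by distance.
; Holding right mouse long enough, then releasing, calls Combine.
; It also drives velocity-based camera lag and handles damage with knockback, respawning and the failure screen.
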(event `InputAxis|MoveRight`
  (params (AxisValue :type "Float (single-precision)"))
  (if (not (`self.bIsInvokeCombine`))
    (if (`self.bInvokeCombine`)
      (`self.AddMovementInput` (`KismetMathLibrary.MakeVector` (* AxisValue 0.3)))
      (else
        (`self.AddMovementInput` (`KismetMathLibrary.MakeVector` AxisValue))))))

(event `InputAction|Jump`
  (params (Key :type "Key Structure"))
  (:`Pressed`
    (if (and (not (`self.bIsInvokeCombine`)) (not (`PawnMovementComponent.IsMoveInputIgnored` (`self.CharacterMovement`))))
      (`self.Jump`))))

(event `self.OnJumped`
  (`GameplayStatics.PlaySoundAtLocation` "/Game/Sound/8BIT_RETRO_Jump_Glide_Up_Dual_Tone_Bright_mono.8BIT_RETRO_Jump_Glide_Up_Dual_Tone_Bright_mono" (`self.K2_GetActorLocation`) (struct) 1.0 1.0 0.0 null null null))

(event `self.ReceiveTick`
  (params (DeltaSeconds :type "Float (single-precision)"))
  (bind (_distance _splitscale) (`self.GetSplitDistance`))
  (bind _returnvalue (`self.K2_GetActorLocation`))
  (bind _camera (`self.Camera`))
  (`|ExecutionSequence`
    (:`then_0`
      (if (`self.bInvokeSplit`)
        (`KismetSystemLibrary.DrawDebugArrow` _returnvalue (+ _returnvalue (* _distance (* _splitscale 400.0))) 0.0 (struct :`G` 1.0 :`B` 0.071448 :`A` 1.0) 0.0 3.0)))
    (:`then_1`
      (`GameplayStatics.SetGlobalTimeDilation` (`KismetMathLibrary.FInterpTo` (`GameplayStatics.GetGlobalTimeDilation`) (`KismetMathLibrary.SelectFloat` 0.1 1.0 (`self.bInvokeSplit`)) DeltaSeconds 20.0)))
    (:`then_2`
      (if (`self.bInvokeCombine`)
        (if (< (`self.InvokeCombineTime`) (`self.CombineTime`))
          (bind _output_get (set `self.InvokeCombineTime` (+ (stale _output_get) DeltaSeconds)))
          (if (> _output_get (`self.CombineTime`))
            (`AudioComponent.Stop` (stale `Key|RightMouseButton` _returnvalue))
            (`GameplayStatics.PlaySound2D` "/Game/Sound/Weapons/8BIT_RETRO_Fire_Blaster_Dirty_High_End_mono.8BIT_RETRO_Fire_Blaster_Dirty_High_End_mono" 1.0 1.0 0.0 null null)))))
    (:`then_3`
      (`SceneComponent.K2_SetRelativeLocation` _camera (`KismetMathLibrary.VInterpTo` (`SceneComponent.RelativeLocation` _camera) (`KismetMathLibrary.ClampVectorSize` (`KismetMathLibrary.InverseTransformDirection` (`SceneComponent.K2_GetComponentToWorld` _camera) (`self.GetVelocity`)) -300.0 300.0) DeltaSeconds 1.0) false false))))

(event `Key|LeftMouseButton`
  (params (Key :type "Key Structure"))
  (bind (_distance _splitscale) (`self.GetSplitDistance`))
  (:`Pressed`
    (`self.SplitBody`
      (:`then`)
      (:`else`
        (set `self.bInvokeSplit` true))))
  (:`Released`
    (if (`self.bInvokeSplit`)
      (set `self.bInvokeSplit` false)
      (`self.Split` (+ (* (`KismetMathLibrary.Normal` _distance) (`CurveFloat.GetFloatValue` (`self.SplitVelocityCurve`) _splitscale)) (`self.GetVelocity`)) _splitscale)
      (`GameplayStatics.PlaySoundAtLocation` "/Game/Sound/Weapons/8BIT_RETRO_Fire_Blaster_Triple_mono.8BIT_RETRO_Fire_Blaster_Triple_mono" (`self.K2_GetActorLocation`) (struct) 1.0 1.0 0.0 null null null))))

(event `Key|RightMouseButton`
  (params (Key :type "Key Structure"))
  (:`Pressed`
    (`self.SplitBody`
      (:`then`
        (set `self.bInvokeCombine` true)
        (set `self.InvokeCombineTime` 0.0)
        (bind _returnvalue (`GameplayStatics.SpawnSoundAttached` "/Game/Sound/hit/8BIT_RETRO_Hit_Bump_Thump_mono.8BIT_RETRO_Hit_Bump_Thump_mono" (`self.RootComponent`) "None" (0.0 0.0 0.0) (struct) "KeepRelativeOffset" false 1.0 1.0 0.0 null null)))
      (:`else`
        (set `self.bInvokeSplit` false))))
  (:`Released`
    (if (`self.bInvokeCombine`)
      (set `self.bInvokeCombine` false)
      (`|ExecutionSequence`
        (:`then_0`
          (if (> (`self.InvokeCombineTime`) (`self.CombineTime`))
            (`self.Combine`)
            (`GameplayStatics.PlaySound2D` "/Game/Sound/Weapons/8BIT_RETRO_Fire_Blaster_Zap_Thud_mono.8BIT_RETRO_Fire_Blaster_Zap_Thud_mono" 1.0 1.0 0.0 null null)))
        (:`then_1`
          (`/Engine/EditorBlueprintResources/StandardMacros.IsValid` _returnvalue
            (:`Is Valid`
              (`AudioComponent.Stop` _returnvalue))))))))

(event `Reborn`
  (`self.K2_SetActorLocation` (`self.RebronLocation`) false true))

(event `DamageAndReborn`
  (bind _output_get (set `self.Health` (- (stale _output_get) 1)))
  (if (> _output_get 0)
    (`self.Reborn`)
    (else
      (`self.Dead`))))

(event `self.ReceivePointDamage`
  (params (Damage :type "Float (single-precision)") (DamageType :type "DamageType Object Reference") (HitLocation :type "Vector Structure") (HitNormal :type "Vector Structure") (HitComponent :type "PrimitiveComponent Object Reference") (BoneName :type Name) (ShotFromDirection :type "Vector Structure") (InstigatedBy :type "Controller Object Reference") (DamageCauser :type "Actor Object Reference") (HitInfo :type "HitResult Structure (by ref)"))
  (bind _returnvalue_x (`KismetMathLibrary.BreakVector` (* ShotFromDirection 1000.0)))
  (`|ExecutionSequence`
    (:`then_0`
      (bind _output_get (set `self.Health` (- (stale _output_get) 1)))
      (if (> _output_get 0)
        (`self.LaunchCharacter` (`KismetMathLibrary.MakeVector` _returnvalue_x 0.0 300.0) true true)
        (else
          (`self.Dead`))))
    (:`then_1`
      (set `self.bCanBeDamaged` false)
      (`KismetSystemLibrary.Delay` 1.0)
      (set `self.bCanBeDamaged` true))
    (:`then_2`
      (`GameplayStatics.PlaySound2D` "/Game/Sound/hit/8BIT_RETRO_Hit_Bump_Zap_mono.8BIT_RETRO_Hit_Bump_Zap_mono" 1.0 1.0 0.0 null null))))

(event `DamageAndCombine`
  (`self.K2_DestroyActor` (`self.SplitBody`))
  (bind _output_get (set `self.Health` (- (stale _output_get) 1)))
  (if (not (> _output_get 0))
    (`self.Dead`)))

(event `Dead`
  (`GameplayStatics.SetGamePaused` true)
  (bind _returnvalue (`|CreateWidget` "/Game/Gameplay/Slime/UI_Failed.UI_Failed_C"))
  (`UserWidget.AddToViewport` _returnvalue 0))

(fn `GetSplitDistance`
  (returns (Distance :type "Vector Structure") (SplitScale :type "Float (double-precision)"))
  (bind _returnvalue (`GameplayStatics.GetPlayerController` 0))
  (bind (_locationx _locationy) (`PlayerController.GetMousePosition` _returnvalue))
  (bind (_worldlocation _worlddirection) (`PlayerController.DeprojectScreenPositionToWorld` _returnvalue _locationx _locationy))
  (bind _returnvalue_2 (- (`.Intersection` (`KismetMathLibrary.LinePlaneIntersection` _worldlocation (+ _worldlocation (* _worlddirection 1000000.0)) (`KismetMathLibrary.MakePlaneFromPointAndNormal` (`self.K2_GetActorLocation`) (0.0 1.0 0.0)))) (`self.K2_GetActorLocation`)))
  (return (`KismetMathLibrary.Normal` _returnvalue_2) (`KismetMathLibrary.MapRangeClamped` (`KismetMathLibrary.VSize` _returnvalue_2) 100.0 400.0 0.2 0.8)))

(fn `UserConstructionScript`)