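; BP_RedCrystal_01 is an environment actor that makes its red crystal mesh bob up and down over time.
; Tick accumulates elapsed time and adds a small sine value of it to the mesh's current world Z each frame, so motion is cumulative and frame-rate dependent.
; The world location is written back as relative location, with the rotation input left unset.
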(event `self.ReceiveBeginPlay`
  (set `self.time` 0.0))

(event `self.ReceiveTick`
  (params (DeltaSeconds :type "Float (single-precision)"))
  (bind _sm_redcrystal_01 (`self.SM_RedCrystal_01`))
  (bind (_returnvalue_x _returnvalue_y _returnvalue_z) (`KismetMathLibrary.BreakVector` (`SceneComponent.K2_GetComponentLocation` _sm_redcrystal_01)))
  (bind _output_get (set `self.time` (+ DeltaSeconds (`self.time`))))
  (`SceneComponent.K2_SetRelativeLocationAndRotation` :`self` _sm_redcrystal_01 :`NewLocation` (`KismetMathLibrary.MakeVector` _returnvalue_x _returnvalue_y (+ (/ (`KismetMathLibrary.Sin` _output_get) 10.0) _returnvalue_z))))

(fn `UserConstructionScript`)